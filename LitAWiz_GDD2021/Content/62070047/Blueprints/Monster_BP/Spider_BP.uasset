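; Spider monster actor that takes damage from fireball hits and dies when its health runs out.
; Overlapping an actor of class FireBall_BP reduces SpiderHP by one.
; Tick polls DeadCheck every frame, destroying the spider once SpiderHP equals exactly zero.
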(event `self.ReceiveTick`
  (params (DeltaSeconds :type "Float (single-precision)"))
  (`self.DeadCheck`))

(event `self.ReceiveActorBeginOverlap`
  (params (OtherActor :type "Actor Object Reference"))
  (if (== (`GameplayStatics.GetObjectClass` OtherActor) "/Game/62070047/Blueprints/Skill_BP/FireBall_BP.FireBall_BP_C")
    (`self.DamageToSpider`)))

(event `DamageToSpider`
  (set `self.Spider_HP` (- (`self.Spider_HP`) 1)))

(event `DeadCheck`
  (if (== (`self.Spider_HP`) 0)
    (`self.K2_DestroyActor`)))

(fn `UserConstructionScript`)