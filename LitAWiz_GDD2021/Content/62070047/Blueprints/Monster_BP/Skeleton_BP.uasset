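; Skeleton monster that chases the player once detected and is destroyed when fireball hits bring its health to zero.
; Find_Range overlap with MainChar sets PlayerInRange, which drives AIMoveTo chasing from Tick, while actor end overlap clears it.
; Capsule overlaps with FireBall_BP subtract fixed damage, and Tick checks for exactly zero HP.
; Reaching the player toggles a CanAttack cooldown and re-chases, but deals no damage here.
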(event `self.CapsuleComponent.OnComponentBeginOverlap`
  (params (OverlappedComponent :type "PrimitiveComponent Object Reference") (OtherActor :type "Actor Object Reference") (OtherComp :type "PrimitiveComponent Object Reference") (OtherBodyIndex :type Integer) (bFromSweep :type Boolean) (SweepResult :type "HitResult Structure (by ref)"))
  (cast `/Game/62070047/Blueprints/Skill_BP/FireBall_BP` OtherActor)
  (`self.DamageToSkeleton` 2))

(event `self.ReceiveTick`
  (params (DeltaSeconds :type "Float (single-precision)"))
  (`self.DeadCheck`)
  (if (`self.PlayerInRange`)
    (`self.Chase Player`)))

(event `DamageToSkeleton`
  (params (Damage :type Integer))
  (set `self.Skeleton_HP` (- (`self.Skeleton_HP`) Damage)))

(event `self.Find_Range.OnComponentBeginOverlap`
  (params (OverlappedComponent :type "PrimitiveComponent Object Reference") (OtherActor :type "Actor Object Reference") (OtherComp :type "PrimitiveComponent Object Reference") (OtherBodyIndex :type Integer) (bFromSweep :type Boolean) (SweepResult :type "HitResult Structure (by ref)"))
  (cast `/Game/62070047/MainChar` OtherActor)
  (set `self.PlayerInRange` true)
  (`self.Chase Player`))

(event `DeadCheck`
  (if (== (`self.Skeleton_HP`) 0)
    (`self.K2_DestroyActor`)))

(event `self.ReceiveActorEndOverlap`
  (params (OtherActor :type "Actor Object Reference"))
  (cast `/Game/62070047/MainChar` OtherActor)
  (set `self.PlayerInRange` false))

(event `Chase Player`
  (`|AIMoveTo` self (0.0 0.0 0.0) (`GameplayStatics.GetPlayerPawn` 0) 1.0
    (:`OnSuccess`
      (if (`self.CanAttack`)
        (set `self.CanAttack` false)
        (`KismetSystemLibrary.Delay` (`self.AttackRate`))
        (set `self.CanAttack` true)
        (if (`self.PlayerInRange`)
          (`self.Chase Player`))
        (else
          (`self.Chase Player`))))))

(fn `UserConstructionScript`)