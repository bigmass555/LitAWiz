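; Web ball projectile for the spider boss that leaves a web where it hits level geometry.
; On overlap with a wall, floor, pressure plate or falling stone, it waits a tiny delay, spawns SpiderWeb_BP at its location and destroys itself.
; Hitting MainChar only destroys it, with no web or damage applied here, and a two-second lifespan removes it otherwise.
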(event `self.ReceiveBeginPlay`
  (`self.SetLifeSpan` 2.0))

(event `self.WebBall.OnComponentBeginOverlap`
  (params (OverlappedComponent :type "PrimitiveComponent Object Reference") (OtherActor :type "Actor Object Reference") (OtherComp :type "PrimitiveComponent Object Reference") (OtherBodyIndex :type Integer) (bFromSweep :type Boolean) (SweepResult :type "HitResult Structure (by ref)"))
  (bind _returnvalue_location (`KismetMathLibrary.BreakTransform` (`self.GetTransform`)))
  (cast `/Game/62070047/Blueprints/Block_BP/Wall_BP` OtherActor
    (:`then`
      (`KismetSystemLibrary.Delay` 0.001 :!label _label)
      (`|SpawnActorFromClass` "/Game/62070047/Blueprints/Block_BP/SpiderWeb_BP.SpiderWeb_BP_C" (`KismetMathLibrary.MakeTransform` _returnvalue_location) "AdjustIfPossibleButAlwaysSpawn" "OverrideRootScale" null null))
    (:`CastFailed`
      (cast `/Game/62070047/Blueprints/Block_BP/Floor_BP` OtherActor
        (:`then`
          (goto _label))
        (:`CastFailed`
          (cast `/Game/62070047/Blueprints/Block_BP/PressurePlate_BP` OtherActor
            (:`then`
              (goto _label))
            (:`CastFailed`
              (cast `/Game/62070047/Blueprints/Skill_BP/StoneFall_BP` OtherActor
                (:`then`
                  (goto _label))
                (:`CastFailed`
                  (cast `/Game/62070047/MainChar` OtherActor)))))))))
  (`self.K2_DestroyActor`))

(fn `UserConstructionScript`)