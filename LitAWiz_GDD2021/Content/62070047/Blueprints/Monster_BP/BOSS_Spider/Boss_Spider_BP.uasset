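; Spider boss that wakes when the player enters its boss area and shoots web balls at them.
; While the player overlaps it, a spawn arrow interpolates toward them, and a Tick-driven Delay paces projectile spawning.
; Rock overlaps on the capsule lower HP, raise the player's hit counter and print boss HP.
; Tick destroys the boss when HP reaches zero.
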(event `self.ReceiveBeginPlay`
  (bind _asmain_char (cast `/Game/62070047/MainChar` (`GameplayStatics.GetPlayerPawn` 0)))
  (set `self.MainChar` _asmain_char))

(event `self.ReceiveTick`
  (params (DeltaSeconds :type "Float (single-precision)"))
  (`self.DeadCheck`)
  (if (`self.BossActivation`)
    (if (`self.PlayerInRange`)
      (`self.Face Player`)
      (`KismetSystemLibrary.Delay` (`self.fire_delay`))
      (`self.Fire WebBall`))
    (else
      (`self.ActivationCheck`))))

(event `DamageToSpider`
  (bind _returnvalue (- (`self.Spider_HP`) 1))
  (set `self.Spider_HP` _returnvalue)
  (bind _asmain_char (cast `/Game/62070047/MainChar` (`GameplayStatics.GetPlayerPawn` 0)))
  (set `/Game/62070047/MainChar.BossSpiderHitCount` (+ (`/Game/62070047/MainChar.BossSpiderHitCount` _asmain_char) 1) _asmain_char)
  (`KismetSystemLibrary.PrintString` (`KismetStringLibrary.Concat_StrStr` "Boss HP : " (`KismetStringLibrary.Conv_IntToString` _returnvalue)))
  (`KismetSystemLibrary.Delay` 1.0))

(event `self.ReceiveActorBeginOverlap`
  (params (OtherActor :type "Actor Object Reference"))
  (cast `/Game/62070047/MainChar` OtherActor)
  (set `self.PlayerInRange` true))

(event `self.CapsuleComponent.OnComponentBeginOverlap`
  (params (OverlappedComponent :type "PrimitiveComponent Object Reference") (OtherActor :type "Actor Object Reference") (OtherComp :type "PrimitiveComponent Object Reference") (OtherBodyIndex :type Integer) (bFromSweep :type Boolean) (SweepResult :type "HitResult Structure (by ref)"))
  (cast `/Game/62070047/Blueprints/Block_BP/Rock_BP` OtherActor)
  (`self.DamageToSpider`))

(event `self.ReceiveActorEndOverlap`
  (params (OtherActor :type "Actor Object Reference"))
  (cast `/Game/62070047/MainChar` OtherActor)
  (set `self.PlayerInRange` false))

(event `DeadCheck`
  (if (== (`self.Spider_HP`) 0)
    (`self.K2_DestroyActor`)))

(event `ActivationCheck`
  (bind _asmain_char (cast `/Game/62070047/MainChar` (`GameplayStatics.GetPlayerPawn` 0)))
  (if (`/Game/62070047/MainChar.InSpiderBossArea` _asmain_char)
    (set `self.BossActivation` true)))

(event `Face Player`
  (bind _webball_spawnarrow (`self.WebBall_SpawnArrow`))
  ;[1 1 1] Arrow Facing to Player
  (`SceneComponent.K2_SetWorldRotation` _webball_spawnarrow (`KismetMathLibrary.RInterpTo` (`SceneComponent.K2_GetComponentRotation` _webball_spawnarrow) (`KismetMathLibrary.FindLookAtRotation` (`SceneComponent.K2_GetComponentLocation` _webball_spawnarrow) (`self.K2_GetActorLocation` (`self.MainChar`))) (`GameplayStatics.GetWorldDeltaSeconds`) 30.0) false false)
  (`KismetSystemLibrary.Delay` 0.001)
  (if (`self.PlayerInRange`)
    (`self.Face Player`)))

(event `Fire WebBall`
  (bind (_returnvalue_location _returnvalue_rotation _returnvalue_scale) (`KismetMathLibrary.BreakTransform` (`SceneComponent.K2_GetComponentToWorld` (`self.WebBall_SpawnArrow`))))
  (`|SpawnActorFromClass` "/Game/62070047/Blueprints/Monster_BP/BOSS_Spider/Boss_Spider_WebBall_BP.Boss_Spider_WebBall_BP_C" (`KismetMathLibrary.MakeTransform` _returnvalue_location _returnvalue_rotation _returnvalue_scale) "Undefined" "OverrideRootScale" null null))

(fn `UserConstructionScript`)