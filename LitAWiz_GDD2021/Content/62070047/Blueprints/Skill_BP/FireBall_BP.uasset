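; Fireball skill actor that destroys itself on hitting level geometry, props or enemies, or when its short life span set at BeginPlay runs out.
; The sphere's begin-overlap runs a chain of casts for wall, floor, pressure plate, spider web and falling stone actors, all sharing one destroy path.
; Skeletons and spiders trigger it only through their capsule component.
; No damage or movement logic appears in these graphs.
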(event `self.ReceiveBeginPlay`
  (`self.SetLifeSpan` 1.0))

(event `self.fireball_sphere.OnComponentBeginOverlap`
  (params (OverlappedComponent :type "PrimitiveComponent Object Reference") (OtherActor :type "Actor Object Reference") (OtherComp :type "PrimitiveComponent Object Reference") (OtherBodyIndex :type Integer) (bFromSweep :type Boolean) (SweepResult :type "HitResult Structure (by ref)"))
  (cast `/Game/62070047/Blueprints/Block_BP/Wall_BP` OtherActor
    (:`then`
      (`KismetSystemLibrary.PrintString` "destroy fireball" false true (struct :`R` 1.0 :`A` 1.0) :!label _label)
      (`self.K2_DestroyActor`))
    (:`CastFailed`
      (cast `/Game/62070047/Blueprints/Block_BP/Floor_BP` OtherActor
        (:`then`
          (goto _label))
        (:`CastFailed`
          (cast `/Game/62070047/Blueprints/Block_BP/PressurePlate_BP` OtherActor
            (:`then`
              (goto _label))
            (:`CastFailed`
              (cast `/Game/62070047/Blueprints/Block_BP/SpiderWeb_BP` OtherActor
                (:`then`
                  (goto _label))
                (:`CastFailed`
                  (cast `/Game/62070047/Blueprints/Skill_BP/StoneFall_BP` OtherActor
                    (:`then`
                      (goto _label))
                    (:`CastFailed`
                      (bind _asskeleton_bp (cast `/Game/62070047/Blueprints/Monster_BP/Skeleton_BP` OtherActor)
                        (:`then`
                          (if (== OtherComp (`Character.CapsuleComponent` _asskeleton_bp))
                            (goto _label)))
                        (:`CastFailed`
                          (bind _asspider_bp (cast `/Game/62070047/Blueprints/Monster_BP/Spider_BP` OtherActor))
                          (if (== OtherComp (`Character.CapsuleComponent` _asspider_bp))
                            (goto _label)))))))))))))))

(fn `UserConstructionScript`)