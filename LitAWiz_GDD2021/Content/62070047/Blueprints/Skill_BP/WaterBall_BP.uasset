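; WaterBall_BP is a short-lived water ball skill actor that destroys itself after one second or on hitting certain objects.
; Its sphere's overlap event runs a chain of casts, destroying the ball on walls, floors, pressure plates, spider webs and falling-stone actors.
; On floors it first waits a tiny delay and spawns a WateredFloor_BP at its own location.
; Other overlapped actors are ignored.
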(event `self.ReceiveBeginPlay`
  (`self.SetLifeSpan` 1.0))

(event `self.WaterBall_Sphere.OnComponentBeginOverlap`
  (params (OverlappedComponent :type "PrimitiveComponent Object Reference") (OtherActor :type "Actor Object Reference") (OtherComp :type "PrimitiveComponent Object Reference") (OtherBodyIndex :type Integer) (bFromSweep :type Boolean) (SweepResult :type "HitResult Structure (by ref)"))
  (bind _returnvalue_location (`KismetMathLibrary.BreakTransform` (`self.GetTransform`)))
  (cast `/Game/62070047/Blueprints/Block_BP/Wall_BP` OtherActor
    (:`then`
      _)
    (:`CastFailed`
      (cast `/Game/62070047/Blueprints/Block_BP/Floor_BP` OtherActor
        (:`then`
          (`KismetSystemLibrary.Delay` 0.001)
          (`|SpawnActorFromClass` "/Game/62070047/Blueprints/Skill_BP/WateredFloor_BP.WateredFloor_BP_C" (`KismetMathLibrary.MakeTransform` _returnvalue_location) "AlwaysSpawn" "OverrideRootScale" null null))
        (:`CastFailed`
          (cast `/Game/62070047/Blueprints/Block_BP/PressurePlate_BP` OtherActor
            (:`then`
              _)
            (:`CastFailed`
              (cast `/Game/62070047/Blueprints/Block_BP/SpiderWeb_BP` OtherActor
                (:`then`
                  _)
                (:`CastFailed`
                  (cast `/Game/62070047/Blueprints/Skill_BP/StoneFall_BP` OtherActor)))))))))
  (`KismetSystemLibrary.PrintString` "destroy waterball" false true (struct :`R` 1.0 :`A` 1.0))
  (`self.K2_DestroyActor`))

(fn `UserConstructionScript`)