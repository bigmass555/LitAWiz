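; WateredFloor_BP is a temporary water puddle skill actor that slows enemies and expires after a ten-second lifespan.
; Overlapping the WaterFloor component divides a Skeleton_BP or Spider_BP's MaxWalkSpeed by SlowSpeedDivider.
; Ending the overlap multiplies the speed back by the same value.
; CheckSparkBall_Box detects SparkBall_BP overlaps through a cast, but nothing follows it yet.
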(event `self.ReceiveBeginPlay`
  (`self.SetLifeSpan` 10.0))

(event `self.WaterFloor.OnComponentBeginOverlap`
  (params (OverlappedComponent :type "PrimitiveComponent Object Reference") (OtherActor :type "Actor Object Reference") (OtherComp :type "PrimitiveComponent Object Reference") (OtherBodyIndex :type Integer) (bFromSweep :type Boolean) (SweepResult :type "HitResult Structure (by ref)"))
  (bind _asskeleton_bp (cast `/Game/62070047/Blueprints/Monster_BP/Skeleton_BP` OtherActor)
    (:`then`
      (bind _charactermovement (`Character.CharacterMovement` _asskeleton_bp))
      (set `CharacterMovementComponent.MaxWalkSpeed` (/ (`CharacterMovementComponent.MaxWalkSpeed` _charactermovement) (`self.SlowSpeedDivider`)) _charactermovement))
    (:`CastFailed`
      (bind _asspider_bp (cast `/Game/62070047/Blueprints/Monster_BP/Spider_BP` OtherActor))
      (bind _charactermovement_2 (`Character.CharacterMovement` _asspider_bp))
      (set `CharacterMovementComponent.MaxWalkSpeed` (/ (`CharacterMovementComponent.MaxWalkSpeed` _charactermovement_2) (`self.SlowSpeedDivider`)) _charactermovement_2))))

(event `self.WaterFloor.OnComponentEndOverlap`
  (params (OverlappedComponent :type "PrimitiveComponent Object Reference") (OtherActor :type "Actor Object Reference") (OtherComp :type "PrimitiveComponent Object Reference") (OtherBodyIndex :type Integer))
  (bind _asskeleton_bp (cast `/Game/62070047/Blueprints/Monster_BP/Skeleton_BP` OtherActor)
    (:`then`
      (bind _charactermovement (`Character.CharacterMovement` _asskeleton_bp))
      (set `CharacterMovementComponent.MaxWalkSpeed` (* (`CharacterMovementComponent.MaxWalkSpeed` _charactermovement) (`self.SlowSpeedDivider`)) _charactermovement))
    (:`CastFailed`
      (bind _asspider_bp (cast `/Game/62070047/Blueprints/Monster_BP/Spider_BP` OtherActor))
      (bind _charactermovement_2 (`Character.CharacterMovement` _asspider_bp))
      (set `CharacterMovementComponent.MaxWalkSpeed` (* (`CharacterMovementComponent.MaxWalkSpeed` _charactermovement_2) (`self.SlowSpeedDivider`)) _charactermovement_2))))

(event `self.CheckSparkBall_Box.OnComponentBeginOverlap`
  (params (OverlappedComponent :type "PrimitiveComponent Object Reference") (OtherActor :type "Actor Object Reference") (OtherComp :type "PrimitiveComponent Object Reference") (OtherBodyIndex :type Integer) (bFromSweep :type Boolean) (SweepResult :type "HitResult Structure (by ref)"))
  (cast `/Game/62070047/Blueprints/Skill_BP/SparkBall_BP` OtherActor))

(fn `UserConstructionScript`)