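; SparkBall is a short-lived skill actor that damages skeletons on overlap and removes itself after a few seconds.
; It records hit enemies by object name in SparkedEnemy, so each skeleton capsule is damaged only once.
; The spider branch inverts that check, calling DamageToSpider with zero damage only for already-recorded spiders.
; A cast chain destroys the ball on floors, stone falls, the boss exit door and pressure-plate or electric-charger doors.
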(event `self.ReceiveBeginPlay`
  (`self.SetLifeSpan` 3.0))

(event `self.SparkBall_Sphere.OnComponentBeginOverlap`
  (params (OverlappedComponent :type "PrimitiveComponent Object Reference") (OtherActor :type "Actor Object Reference") (OtherComp :type "PrimitiveComponent Object Reference") (OtherBodyIndex :type Integer) (bFromSweep :type Boolean) (SweepResult :type "HitResult Structure (by ref)"))
  (bind _sparkedenemy (`self.SparkedEnemy`))
  (bind _asskeleton_bp (cast `/Game/62070047/Blueprints/Monster_BP/Skeleton_BP` OtherActor)
    (:`then`
      (if (== OtherComp (`Character.CapsuleComponent` _asskeleton_bp))
        (bind _returnvalue (`KismetSystemLibrary.GetObjectName` _asskeleton_bp))
        (if (not (`KismetArrayLibrary.Array_Contains` _sparkedenemy _returnvalue))
          (`/Game/62070047/Blueprints/Monster_BP/Skeleton_BP.DamageToSkeleton` _asskeleton_bp 1)
          (`KismetArrayLibrary.Array_Add` _sparkedenemy _returnvalue :!label _label))))
    (:`CastFailed`
      (bind _asspider_bp (cast `/Game/62070047/Blueprints/Monster_BP/Spider_BP` OtherActor)
        (:`then`
          (if (== OtherComp (`Character.CapsuleComponent` _asspider_bp))
            (if (`KismetArrayLibrary.Array_Contains` (`self.SparkedEnemy`) (`KismetSystemLibrary.GetObjectName` _asspider_bp))
              (`/Game/62070047/Blueprints/Monster_BP/Spider_BP.DamageToSpider` _asspider_bp 0)
              (goto _label))))
        (:`CastFailed`
          (cast `/Game/62070047/Blueprints/Block_BP/Floor_BP` OtherActor
            (:`then`
              (`self.K2_DestroyActor` :!label _label_2))
            (:`CastFailed`
              (bind _aspressure_plate_bp (cast `/Game/62070047/Blueprints/Block_BP/PressurePlate_BP` OtherActor)
                (:`then`
                  (if (== (`/Game/62070047/Blueprints/Block_BP/PressurePlate_BP.SlideDoor` _aspressure_plate_bp) OtherComp)
                    (goto _label_2)))
                (:`CastFailed`
                  (cast `/Game/62070047/Blueprints/Monster_BP/BOSS_Spider/Boss_Spider_ExitDoor` OtherActor
                    (:`then`
                      (goto _label_2))
                    (:`CastFailed`
                      (cast `/Game/62070047/Blueprints/Skill_BP/StoneFall_BP` OtherActor
                        (:`then`
                          (goto _label_2))
                        (:`CastFailed`
                          (bind _aselectric_charger_bp (cast `/Game/62070047/Blueprints/Block_BP/ElectricCharger_BP` OtherActor))
                          (if (== (`/Game/62070047/Blueprints/Block_BP/ElectricCharger_BP.ironDoor` _aselectric_charger_bp) OtherComp)
                            (goto _label_2)))))))))))))))

(fn `UserConstructionScript`)