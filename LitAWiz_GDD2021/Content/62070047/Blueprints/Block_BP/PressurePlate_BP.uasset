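; Pressure plate puzzle block that slides a door open while the main character, a falling stone or a rock rests on it.
; An overlap counter keeps it active until empty; after a retriggerable delay, the plate snaps down by dividing its world Z, or back to default.
; Tick steps the door along world Z or Y toward its offset or start position at a frame-rate-dependent speed.
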(event `self.ReceiveBeginPlay`
  (set `self.Default_Plate_Location` (`SceneComponent.K2_GetComponentLocation` (`self.StonePressurePlate`)))
  (set `self.Default_Door_Location` (`SceneComponent.K2_GetComponentLocation` (`self.SlideDoor`))))

(event `self.StonePressurePlate.OnComponentBeginOverlap`
  (params (OverlappedComponent :type "PrimitiveComponent Object Reference") (OtherActor :type "Actor Object Reference") (OtherComp :type "PrimitiveComponent Object Reference") (OtherBodyIndex :type Integer) (bFromSweep :type Boolean) (SweepResult :type "HitResult Structure (by ref)"))
  (bind _returnvalue (`GameplayStatics.GetObjectClass` OtherActor))
  (if (or (== _returnvalue "/Game/62070047/MainChar.MainChar_C") (== _returnvalue "/Game/62070047/Blueprints/Skill_BP/StoneFall_BP.StoneFall_BP_C") (== _returnvalue "/Game/62070047/Blueprints/Block_BP/Rock_BP.Rock_BP_C"))
    (bind _output_get (set `self.OverlapCount` (+ (`self.OverlapCount`) 1)))
    (`KismetSystemLibrary.PrintString` (`KismetStringLibrary.Conv_IntToString` _output_get) false)
    (set `self.IsActive` true)
    (`KismetSystemLibrary.RetriggerableDelay` 0.5)
    (`self.Active`)))

(event `self.StonePressurePlate.OnComponentEndOverlap`
  (params (OverlappedComponent :type "PrimitiveComponent Object Reference") (OtherActor :type "Actor Object Reference") (OtherComp :type "PrimitiveComponent Object Reference") (OtherBodyIndex :type Integer))
  (bind _returnvalue (`GameplayStatics.GetObjectClass` OtherActor))
  (bind _overlapcount (`self.OverlapCount`))
  (if (or (== _returnvalue "/Game/62070047/MainChar.MainChar_C") (== _returnvalue "/Game/62070047/Blueprints/Skill_BP/StoneFall_BP.StoneFall_BP_C") (== _returnvalue "/Game/62070047/Blueprints/Block_BP/Rock_BP.Rock_BP_C"))
    (set `self.OverlapCount` (- _overlapcount 1))
    (if (< _overlapcount 1)
      (set `self.IsActive` false)
      (`KismetSystemLibrary.RetriggerableDelay` 0.5)
      (`self.Deactive`))))

(event `Active`
  (`SceneComponent.K2_SetWorldLocation` (`self.StonePressurePlate`) (`KismetMathLibrary.MakeVector` (.x (`self.Default_Plate_Location`)) (.y (`self.Default_Plate_Location`)) (/ (.z (`self.Default_Plate_Location`)) (`self.MovePlateDownDivider`))) false false))

(event `self.ReceiveTick`
  (params (DeltaSeconds :type "Float (single-precision)"))
  (bind _slidedoor (`self.SlideDoor`))
  (bind _slidedoor_2 (`self.SlideDoor`))
  (bind _slidedoor_3 (`self.SlideDoor`))
  (bind _slidedoor_4 (`self.SlideDoor`))
  (bind _z (.z (`SceneComponent.K2_GetComponentLocation` _slidedoor_4)))
  (bind _z_2 (.z (`SceneComponent.K2_GetComponentLocation` _slidedoor)))
  (bind _y (.y (`SceneComponent.K2_GetComponentLocation` _slidedoor_2)))
  (bind _y_2 (.y (`SceneComponent.K2_GetComponentLocation` _slidedoor_3)))
  (if (`self.IsActive`)
    (if (`self.IsZ-Axiz`)
      (if (< _z_2 (+ (.z (`self.Default_Door_Location`)) (`self.MoveDoorUp`)))
        (`SceneComponent.K2_SetWorldLocation` _slidedoor (`KismetMathLibrary.MakeVector` (.x (`SceneComponent.K2_GetComponentLocation` _slidedoor)) (.y (`SceneComponent.K2_GetComponentLocation` _slidedoor)) (+ _z_2 (`self.MoveDoorSpeed`))) false false))
      (elif (< _y (+ (.y (`self.Default_Door_Location`)) (`self.MoveDoorUp`)))
        (`SceneComponent.K2_SetWorldLocation` _slidedoor_2 (`KismetMathLibrary.MakeVector` (.x (`SceneComponent.K2_GetComponentLocation` _slidedoor_2)) (+ _y (`self.MoveDoorSpeed`)) (.z (`SceneComponent.K2_GetComponentLocation` _slidedoor_2))) false false)))
    (elif (`self.IsZ-Axiz`)
      (if (> _z (.z (`self.Default_Door_Location`)))
        (`SceneComponent.K2_SetWorldLocation` _slidedoor_4 (`KismetMathLibrary.MakeVector` (.x (`SceneComponent.K2_GetComponentLocation` _slidedoor_4)) (.y (`SceneComponent.K2_GetComponentLocation` _slidedoor_4)) (- _z (`self.MoveDoorSpeed`))) false false))
      (elif (> _y_2 (.y (`self.Default_Door_Location`)))
        (`SceneComponent.K2_SetWorldLocation` _slidedoor_3 (`KismetMathLibrary.MakeVector` (.x (`SceneComponent.K2_GetComponentLocation` _slidedoor_3)) (- _y_2 (`self.MoveDoorSpeed`)) (.z (`SceneComponent.K2_GetComponentLocation` _slidedoor_3))) false false)))))

(event `Deactive`
  (`SceneComponent.K2_SetWorldLocation` (`self.StonePressurePlate`) (`self.Default_Plate_Location`) false false))

(fn `UserConstructionScript`)