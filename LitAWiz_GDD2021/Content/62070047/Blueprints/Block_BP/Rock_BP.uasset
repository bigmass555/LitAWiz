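; Rock actor that sticks in spider webs and is destroyed on contact with the spider boss.
; When Rock_incoll overlaps a SpiderWeb_BP, physics on Rock switches off after a short delay; overlapping Boss_Spider_BP's capsule destroys the rock.
; Physics switches back on when Rock itself, rather than Rock_incoll, stops overlapping a web.
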(event `self.Rock_incoll.OnComponentBeginOverlap`
  (params (OverlappedComponent :type "PrimitiveComponent Object Reference") (OtherActor :type "Actor Object Reference") (OtherComp :type "PrimitiveComponent Object Reference") (OtherBodyIndex :type Integer) (bFromSweep :type Boolean) (SweepResult :type "HitResult Structure (by ref)"))
  (if (== (`GameplayStatics.GetObjectClass` OtherActor) "/Game/62070047/Blueprints/Block_BP/SpiderWeb_BP.SpiderWeb_BP_C")
    (`KismetSystemLibrary.Delay` 0.1)
    (`PrimitiveComponent.SetSimulatePhysics` (`self.Rock`) false)
    (else
      (bind _asboss_spider_bp (cast `/Game/62070047/Blueprints/Monster_BP/BOSS_Spider/Boss_Spider_BP` OtherActor))
      (if (== (`Character.CapsuleComponent` _asboss_spider_bp) OtherComp)
        (`self.K2_DestroyActor`)))))

(event `self.Rock.OnComponentEndOverlap`
  (params (OverlappedComponent :type "PrimitiveComponent Object Reference") (OtherActor :type "Actor Object Reference") (OtherComp :type "PrimitiveComponent Object Reference") (OtherBodyIndex :type Integer))
  (if (== (`GameplayStatics.GetObjectClass` OtherActor) "/Game/62070047/Blueprints/Block_BP/SpiderWeb_BP.SpiderWeb_BP_C")
    (`PrimitiveComponent.SetSimulatePhysics` (`self.Rock`) true)))

(fn `UserConstructionScript`)