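; ResetCharger_BP is a stone pressure plate block that resets the level's electric chargers to their initial power state.
; On BeginPlay it records the IsPowerOn flag of every ElectricCharger_BP in an array.
; When MainChar overlaps the plate, it fetches the chargers again and writes back each saved value by array index, relying on the same actor order.
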(event `self.ReceiveBeginPlay`
  (bind _outactors (`GameplayStatics.GetAllActorsOfClass` "/Game/62070047/Blueprints/Block_BP/ElectricCharger_BP.ElectricCharger_BP_C"))
  (for _array_element _outactors
    (`KismetArrayLibrary.Array_Add` (`self.List_ChargerPowerState`) (`/Game/62070047/Blueprints/Block_BP/ElectricCharger_BP.IsPowerOn` _array_element))))

(event `self.StonePressurePlate.OnComponentBeginOverlap`
  (params (OverlappedComponent :type "PrimitiveComponent Object Reference") (OtherActor :type "Actor Object Reference") (OtherComp :type "PrimitiveComponent Object Reference") (OtherBodyIndex :type Integer) (bFromSweep :type Boolean) (SweepResult :type "HitResult Structure (by ref)"))
  (cast `/Game/62070047/MainChar` OtherActor)
  (bind _outactors (`GameplayStatics.GetAllActorsOfClass` "/Game/62070047/Blueprints/Block_BP/ElectricCharger_BP.ElectricCharger_BP_C"))
  (for (_array_element _array_index) _outactors
    (set `/Game/62070047/Blueprints/Block_BP/ElectricCharger_BP.IsPowerOn` (`|GetArrayItem` (`self.List_ChargerPowerState`) _array_index) _array_element)))

(fn `UserConstructionScript`)