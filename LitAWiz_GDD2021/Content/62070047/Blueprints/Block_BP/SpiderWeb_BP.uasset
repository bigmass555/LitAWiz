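; Spider web block that slows the player while overlapped and burns away when hit by a fireball.
; Begin overlap with MainChar divides walk speed and jump velocity by SpeedDecreser and halves animation rate; end overlap reverses this.
; While the player is inside, Tick repeatedly divides vertical velocity by the same factor, a frame-rate-dependent damping.
; FireBall_BP overlap triggers Onfire, which swaps to a burning material and destroys the web after a short delay.
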(event `self.ReceiveTick`
  (params (DeltaSeconds :type "Float (single-precision)"))
  (if (`self.IsPlayerIn`)
    (bind _charactermovement (`Character.CharacterMovement` (stale `self.SpiderWeb.OnComponentBeginOverlap` _asmain_char)))
    (set `MovementComponent.Velocity` (`KismetMathLibrary.MakeVector` (.x (`MovementComponent.Velocity` _charactermovement)) (.y (`MovementComponent.Velocity` _charactermovement)) (/ (.z (`MovementComponent.Velocity` _charactermovement)) (`self.SpeedDecreser`))) _charactermovement)))

(event `self.SpiderWeb.OnComponentBeginOverlap`
  (params (OverlappedComponent :type "PrimitiveComponent Object Reference") (OtherActor :type "Actor Object Reference") (OtherComp :type "PrimitiveComponent Object Reference") (OtherBodyIndex :type Integer) (bFromSweep :type Boolean) (SweepResult :type "HitResult Structure (by ref)"))
  (bind _returnvalue (`GameplayStatics.GetObjectClass` OtherActor))
  (bind _speeddecreser (`self.SpeedDecreser`))
  (if (== _returnvalue "/Game/62070047/MainChar.MainChar_C")
    (bind _asmain_char (cast `/Game/62070047/MainChar` (`GameplayStatics.GetPlayerPawn` 0)))
    (bind _charactermovement (`Character.CharacterMovement` _asmain_char))
    (set `CharacterMovementComponent.MaxWalkSpeed` (/ (`CharacterMovementComponent.MaxWalkSpeed` _charactermovement) _speeddecreser) _charactermovement)
    (set `CharacterMovementComponent.JumpZVelocity` (/ (`CharacterMovementComponent.JumpZVelocity` _charactermovement) _speeddecreser) _charactermovement)
    (set `self.IsPlayerIn` true)
    (bind _mesh (`Character.Mesh` _asmain_char))
    (set `SkeletalMeshComponent.GlobalAnimRateScale` (/ (`SkeletalMeshComponent.GlobalAnimRateScale` _mesh) 2.0) _mesh)
    (elif (== _returnvalue "/Game/62070047/Blueprints/Skill_BP/FireBall_BP.FireBall_BP_C")
      (`self.Onfire`))))

(event `self.SpiderWeb.OnComponentEndOverlap`
  (params (OverlappedComponent :type "PrimitiveComponent Object Reference") (OtherActor :type "Actor Object Reference") (OtherComp :type "PrimitiveComponent Object Reference") (OtherBodyIndex :type Integer))
  (bind _speeddecreser (`self.SpeedDecreser`))
  (if (== (`GameplayStatics.GetObjectClass` OtherActor) "/Game/62070047/MainChar.MainChar_C")
    (bind _asmain_char (cast `/Game/62070047/MainChar` (`GameplayStatics.GetPlayerPawn` 0)))
    (bind _charactermovement (`Character.CharacterMovement` _asmain_char))
    (set `CharacterMovementComponent.MaxWalkSpeed` (* (`CharacterMovementComponent.MaxWalkSpeed` _charactermovement) _speeddecreser) _charactermovement)
    (set `CharacterMovementComponent.JumpZVelocity` (* (`CharacterMovementComponent.JumpZVelocity` _charactermovement) _speeddecreser) _charactermovement)
    (set `self.IsPlayerIn` false)
    (bind _mesh (`Character.Mesh` (stale `self.SpiderWeb.OnComponentBeginOverlap` _asmain_char)))
    (set `SkeletalMeshComponent.GlobalAnimRateScale` (* (`SkeletalMeshComponent.GlobalAnimRateScale` _mesh) 2.0) _mesh)))

(event `Onfire`
  (`PrimitiveComponent.SetMaterial` (`self.SpiderWeb`) 0 (`self.onfire_matREF`))
  (`KismetSystemLibrary.Delay` 1.5)
  (`self.K2_DestroyActor`))

(fn `UserConstructionScript`)