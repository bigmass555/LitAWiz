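; ElectricCharger_BP is a switch block that toggles power when a SparkBall_BP overlaps its Charger, driving a sliding IronDoor.
; Tick sets the Charger material to show the power state and steps the door along world X between its BeginPlay position and an offset of SlideXby in the negative direction.
; Power normally moves the door toward the offset, while InvertPower reverses that mapping.
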(event `self.ReceiveBeginPlay`
  (bind _returnvalue_x (`KismetMathLibrary.BreakVector` (`SceneComponent.K2_GetComponentLocation` (`self.ironDoor`))))
  (set `self.DefualtDoorLocationX` _returnvalue_x))

(event `self.ReceiveTick`
  (params (DeltaSeconds :type "Float (single-precision)"))
  (bind (_returnvalue_x _returnvalue_y _returnvalue_z) (`KismetMathLibrary.BreakVector` (`SceneComponent.K2_GetComponentLocation` (`self.ironDoor`))))
  (bind (_returnvalue_x_2 _returnvalue_y_2 _returnvalue_z_2) (`KismetMathLibrary.BreakVector` (`SceneComponent.K2_GetComponentLocation` (`self.ironDoor`))))
  (if (`self.InvertPower`)
    (if (`self.IsPowerOn`)
      (`PrimitiveComponent.SetMaterial` (`self.charger`) 0 (`self.refmat_powerOn`))
      (if (< _returnvalue_x_2 (`self.DefualtDoorLocationX`)) :!label _label
        (`SceneComponent.K2_SetWorldLocation` (`self.ironDoor`) (`KismetMathLibrary.MakeVector` (+ _returnvalue_x_2 (`self.DoorSlideSpeed`)) _returnvalue_y_2 _returnvalue_z_2) false false))
      (else
        (`PrimitiveComponent.SetMaterial` (`self.charger`) 0 (`self.refmat_powerOff`))
        (if (> _returnvalue_x (- (`self.DefualtDoorLocationX`) (`self.SlideXby`))) :!label _label_2
          (`SceneComponent.K2_SetWorldLocation` (`self.ironDoor`) (`KismetMathLibrary.MakeVector` (- _returnvalue_x (`self.DoorSlideSpeed`)) _returnvalue_y _returnvalue_z) false false))))
    (elif (`self.IsPowerOn`)
      (`PrimitiveComponent.SetMaterial` (`self.charger`) 0 (`self.refmat_powerOn`))
      (goto _label_2)
      (else
        (`PrimitiveComponent.SetMaterial` (`self.charger`) 0 (`self.refmat_powerOff`))
        (goto _label)))))

(event `self.charger.OnComponentBeginOverlap`
  (params (OverlappedComponent :type "PrimitiveComponent Object Reference") (OtherActor :type "Actor Object Reference") (OtherComp :type "PrimitiveComponent Object Reference") (OtherBodyIndex :type Integer) (bFromSweep :type Boolean) (SweepResult :type "HitResult Structure (by ref)"))
  (cast `/Game/62070047/Blueprints/Skill_BP/SparkBall_BP` OtherActor)
  (if (`self.IsPowerOn`)
    (set `self.IsPowerOn` false)
    (else
      (set `self.IsPowerOn` true))))

(fn `UserConstructionScript`)